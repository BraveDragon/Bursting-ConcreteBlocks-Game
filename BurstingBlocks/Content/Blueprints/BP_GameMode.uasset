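; BP_GameMode is the game mode that creates and centrally updates the HUD showing player and enemy HP.
; On BeginPlay it creates WBP_UI with a maximum player HP and adds it to the viewport.
; Every Tick it passes StaticBlocks as the player HP, then looks up BP_Kraken with GetActorOfClass and pushes its HP and MaxHP to the enemy display.
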(event `self.ReceiveBeginPlay`
  (bind _returnvalue (`|CreateWidget` "/Game/Blueprints/WBP_UI.WBP_UI_C")) ; UIオブジェクトを生成
  (bind _output_get (set `self.UI` _returnvalue))
  (`UserWidget.AddToViewport` _output_get 0) ; UIを画面に追加
)

(event `self.ReceiveTick`
  (params (DeltaSeconds :type "Float (single-precision)"))
  (`/Game/Blueprints/WBP_UI.UpdatePlayerHP` (`self.UI`) (`self.StaticBlocks`))
  (bind _returnvalue (`GameplayStatics.GetActorOfClass` "/Game/Blueprints/BP_Kraken.BP_Kraken_C"))
  (`/Game/Blueprints/WBP_UI.UpdateEnemyHP` (`self.UI`) (`/Game/Blueprints/BP_Kraken.HP` _returnvalue) (`/Game/Blueprints/BP_Kraken.MaxHP` _returnvalue)))

(fn `UserConstructionScript`)