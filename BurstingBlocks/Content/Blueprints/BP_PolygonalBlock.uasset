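; BP_PolygonalBlock is a destructible block actor that homes in on player pawn 0 horizontally at a set velocity.
; Tick moves it without sweep, and overlapping a BP_Wall or another BP_PolygonalBlock switches its mesh to Static mobility, clears Movable and increments BP_GameMode's StaticBlocks count.
; Any damage spawns an explosion effect and sound, decrements that count if the block is no longer movable, then destroys it.
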(event `self.ReceiveBeginPlay`)

(event `self.ReceiveTick`
  (params (DeltaSeconds :type "Float (single-precision)"))
  (bind _velocity (`self.Velocity`))
  (`self.K2_SetActorLocation` (+ (`self.K2_GetActorLocation`) (* (* DeltaSeconds (`KismetMathLibrary.Normal` (- (`self.K2_GetActorLocation` (`GameplayStatics.GetPlayerPawn` 0)) (`self.K2_GetActorLocation`)))) (`KismetMathLibrary.MakeVector` _velocity _velocity)))))

(event `self.ReceiveAnyDamage`
  (params (Damage :type "Float (single-precision)") (DamageType :type "DamageType Object Reference") (InstigatedBy :type "Controller Object Reference") (DamageCauser :type "Actor Object Reference"))
  (bind (_returnvalue_location _returnvalue_rotation) (`KismetMathLibrary.BreakTransform` (`self.GetTransform`)))
  (`GameplayStatics.SpawnEmitterAtLocation` "/Game/StarterContent/Particles/P_Explosion.P_Explosion" _returnvalue_location _returnvalue_rotation (8.0 8.0 8.0))
  (`GameplayStatics.SpawnSoundAtLocation` "/Game/StarterContent/Audio/Explosion01.Explosion01" (`self.K2_GetActorLocation`) (struct) 1.0 1.0 0.0 null null)
  (if (== (`self.Movable`) false)
    (bind _returnvalue (`GameplayStatics.GetActorOfClass` "/Game/Blueprints/BP_GameMode.BP_GameMode_C"))
    (`/Engine/EditorBlueprintResources/StandardMacros.DecrementInt` (`/Game/Blueprints/BP_GameMode.StaticBlocks` _returnvalue)
      (:`  `
        _)))
  (`self.K2_DestroyActor`))

(event `self.ReceiveActorBeginOverlap`
  (params (OtherActor :type "Actor Object Reference"))
  (cast `/Game/Megascans/3D_Assets/Castle_Wall_sbxuw/BP_Wall` OtherActor
    (:`then`
      _)
    (:`CastFailed`
      (cast `/Game/Blueprints/BP_PolygonalBlock` OtherActor)))
  (`SceneComponent.SetMobility` (`self.Block`) "Static")
  (set `self.Movable` false)
  (bind _returnvalue (`GameplayStatics.GetActorOfClass` "/Game/Blueprints/BP_GameMode.BP_GameMode_C"))
  (`/Engine/EditorBlueprintResources/StandardMacros.IncrementInt` (`/Game/Blueprints/BP_GameMode.StaticBlocks` _returnvalue)))

(fn `UserConstructionScript`)