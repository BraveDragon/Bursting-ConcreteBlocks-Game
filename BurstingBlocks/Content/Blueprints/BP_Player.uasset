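; BP_Player is the player-controlled actor that slides sideways, rotates and fires bullets.
; Enhanced Input drives movement along world Y within fixed limits through IsAbleToMove, and rotation, both scaled by delta time for frame-rate independence.
; Fire spawns a BP_Bullet at the Scene component's world transform.
; The IsAbleToRotate limit check is left unwired, so rotation is unclamped.
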(event `self.ReceiveBeginPlay`
  (`self.EnableInput` (`GameplayStatics.GetPlayerController` 0)))

(event `EnhancedInput|/Game/IA_Move`
  (params (ActionValue :type "Float (double-precision)") (ElapsedSeconds :type "Float (double-precision)") (TriggeredSeconds :type "Float (double-precision)") (InputAction :type "InputAction Object Reference" :default "/Game/IA_Move.IA_Move"))
  (bind _returnvalue (`self.K2_GetActorLocation`))
  (bind _returnvalue_2 (* (`GameplayStatics.GetWorldDeltaSeconds`) (* ActionValue 200.0)))
  (:`Triggered`
    (bind _answer (`self.IsAbleToMove` -2688.0 -2580.0 _returnvalue_2 _returnvalue))
    (if _answer
      (`self.K2_SetActorLocation` (+ (`KismetMathLibrary.MakeVector` 0.0 _returnvalue_2) _returnvalue)))))

(event `EnhancedInput|/Game/IA_Rotate`
  (params (ActionValue :type "Float (double-precision)") (ElapsedSeconds :type "Float (double-precision)") (TriggeredSeconds :type "Float (double-precision)") (InputAction :type "InputAction Object Reference" :default "/Game/IA_Rotate.IA_Rotate"))
  (:`Triggered`
    (`self.K2_SetActorRotation` (`KismetMathLibrary.Conv_VectorToRotator` (+ (`KismetMathLibrary.MakeVector` 0.0 0.0 (* (`GameplayStatics.GetWorldDeltaSeconds`) (* ActionValue 1.0))) (`self.K2_GetActorRotation`))))))

(event `EnhancedInput|/Game/IA_Fire`
  (params (ActionValue :type Boolean) (ElapsedSeconds :type "Float (double-precision)") (TriggeredSeconds :type "Float (double-precision)") (InputAction :type "InputAction Object Reference" :default "/Game/IA_Fire.IA_Fire"))
  (:`Started`
    (`|SpawnActorFromClass` "/Game/Blueprints/BP_Bullet.BP_Bullet_C" (`SceneComponent.K2_GetComponentToWorld` (`self.Scene`)) "Undefined" "OverrideRootScale" null null)))

(fn `IsAbleToMove`
  (params (LeftLimit :type "Float (double-precision)") (RightLimit :type "Float (double-precision)") (Direction :type "Float (double-precision)") (Position :type "Vector Structure"))
  (returns (answer :type Boolean))
  (bind _returnvalue (+ Direction Position_Y))
  (return (and (< LeftLimit _returnvalue) (> RightLimit _returnvalue))))

(fn `IsAbleToRotate`
  (params (UpLimit :type "Float (double-precision)") (DownLimit :type "Float (double-precision)") (Direction :type "Float (double-precision)") (Rotation :type "Rotator Structure"))
  (returns (answer :type Boolean))
  (bind _returnvalue (+ Direction Rotation_Roll))
  (return (and (< UpLimit _returnvalue) (> DownLimit _returnvalue))))

(fn `UserConstructionScript`)